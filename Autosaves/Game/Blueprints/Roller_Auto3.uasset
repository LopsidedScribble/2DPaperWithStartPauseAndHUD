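; Roller is a moving enemy hazard that knocks back and damages the player character on contact.
; The construction script feeds four relative points, PointA to PointD, into the BasicEnemyMove interp movement as its path.
; When the Sphere overlaps a MyCharacter, it applies damage and launches the character upward and along X, using the sweep normal's X for horizontal direction and overriding existing velocity.
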(event OnComponentBeginOverlap(Sphere)
  (params (OverlappedComponent :type Primitive%20Component%20Object%20Reference) (OtherActor :type Actor%20Object%20Reference) (OtherComp :type Primitive%20Component%20Object%20Reference) (OtherBodyIndex :type Integer) (bFromSweep :type Boolean) (SweepResult :type Hit%20Result%20Structure%20%28by%20ref%29))
  (bind _asmy_character (Utilities|Casting|CastToMyCharacter OtherActor))
  (Character|LaunchCharacter _asmy_character (Math|Vector|MakeVector (* (.x (.Normal (Collision|BreakHitResult SweepResult))) -1e+03) 0.0 4e+02) true true)
  (Game|Damage|ApplyDamage _asmy_character 1e+01 0 0 "/Script/Engine.DamageType"))

(event EventBeginPlay)

(event Collision|EventActorBeginOverlap
  (params (OtherActor :type Actor%20Object%20Reference)))

(event EventTick
  (params (DeltaSeconds :type Float%20%28single-precision%29)))

(fn ConstructionScript
  (Variables|/Script/Engine.InterpToMovementComponent|SetControlPoints (Variables|Default|GetBasicEnemyMove) (Utilities|Array|MakeArray (Utilities|Struct|MakeInterpControlPoint (Variables|Default|GetPoint%20A) true) (Utilities|Struct|MakeInterpControlPoint (Variables|Default|GetPoint%20B) true) (Utilities|Struct|MakeInterpControlPoint (Variables|Default|GetPoint%20C) true) (Utilities|Struct|MakeInterpControlPoint (Variables|Default|GetPoint%20D) true))))